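; BP_Doux is the Doux character Blueprint, which shows a line-by-line dialogue on screen.
; Each DouxDialogue event advances an index into the DDialogue array and writes that line to a WB_DouxDialogue widget, hiding its DouxBase element on odd indices.
; If the widget is missing, the event only creates and displays it.
; Once the index passes the last line, the widget is removed from the screen.
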(event `/Game/Levels/Level_2/BPI_Doux.DouxDialogue`
  (bind _d_talkindex (`self.D_TalkIndex`))
  (`/Engine/EditorBlueprintResources/StandardMacros.IncrementInt` _d_talkindex
    (:`  `
      (if (< _d_talkindex (`KismetArrayLibrary.Array_Length` (`self.D_Dialogue`)))
        (`self.DouxUI`
          (:`then`
            (`TextBlock.SetText` (`/Game/Levels/Level_2/WB_DouxDialogue.DouxText` (`self.DouxUI`)) (`KismetTextLibrary.Conv_StringToText` (`|GetArrayItem` (`self.D_Dialogue`) (`self.D_TalkIndex`))))
            (if (> (mod (`self.D_TalkIndex`) 2) 0)
              (set `Widget.Visibility` "Hidden" (`/Game/Levels/Level_2/WB_DouxDialogue.DouxBase` (`self.DouxUI`)))
              (else
                (set `Widget.Visibility` "Visible" (`/Game/Levels/Level_2/WB_DouxDialogue.DouxBase` (`self.DouxUI`))))))
          (:`else`
            (bind _returnvalue (`|CreateWidget` "/Game/Levels/Level_2/WB_DouxDialogue.WB_DouxDialogue_C" (`GameplayStatics.GetPlayerController` 0)))
            (bind _output_get (set `self.DouxUI` _returnvalue))
            (`UserWidget.AddToViewport` _output_get 0)))
        (else
          (`Widget.RemoveFromParent` (`self.DouxUI`)))))))

(fn `UserConstructionScript`)