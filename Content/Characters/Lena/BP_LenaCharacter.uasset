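; BP_LenaCharacter is Lena, a side-scrolling flipbook character who moves, jumps, shoots, collects a key and talks to NPCs.
; Tick picks gun or unarmed flipbooks from movement state, hides Duckie once dead, and flips control rotation by X velocity.
; Z fires projectiles when armed, throttled by a delay.
; E messages overlapping villagers and Doux through dialogue interfaces, flagging the Doux conversation, while capsule overlap detects the key.
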(event `Key|Z`
  (params (Key :type "Key Structure"))
  ;[1 1 1] Firing the gun
  (:`Pressed`
    (if (`self.HaveGun`)
      (if (not (`self.HasFired`))
        (`|SpawnActorFromClass` "/Game/Characters/Lena/BP_GunProjectile.BP_GunProjectile_C" (`SceneComponent.K2_GetComponentToWorld` (`self.GunShootPoint`)) "Undefined" "OverrideRootScale" null null)
        (set `self.HasFired` true)
        (`GameplayStatics.PlaySoundAtLocation` "/Game/Sounds/WAV_Shotgun.WAV_Shotgun" (0.0 0.0 0.0) (struct) 1.0 1.0 0.0 null null null null)
        (`KismetSystemLibrary.Delay` 1.2)
        (set `self.HasFired` false)))))

(event `self.ReceiveTick`
  (params (DeltaSeconds :type "Float (single-precision)"))
  ;[1 1 1] animation controllers, rotation and contextual animations
  (`self.UpdateAnimation`)
  (`self.UpdateControlRotation`))

(event `InputAxis|Move Right`
  (params (AxisValue :type "Float (single-precision)"))
  ;[1 1 1] animation controllers, rotation and contextual animations
  (`self.AddMovementInput` (1.0 0.0 0.0) AxisValue)
  (`MovementComponent.SetPlaneConstraintFromVectors` (`self.CharacterMovement`) (0.0 0.0 0.0) (0.0 0.0 0.0)))

(event `InputAction|Jump`
  (params (Key :type "Key Structure"))
  ;[1 1 1] animation controllers, rotation and contextual animations
  (:`Pressed`
    (`self.Jump`)
    (`GameplayStatics.PlaySound2D` "/Game/Sounds/Jump.Jump" 1.0 1.0 0.0 null null))
  (:`Released`
    (`self.StopJumping`)))

(event `UpdateAnimation`
  ;[1 1 1] animation controllers, rotation and contextual animations
  (if (`self.HaveGun`)
    (`PaperFlipbookComponent.SetFlipbook` (`self.Sprite`) (select `bool` (`NavMovementComponent.IsFalling` (`self.CharacterMovement`)) :`false` (select `bool` (> (`KismetMathLibrary.VSize` (`MovementComponent.Velocity` (`self.CharacterMovement`))) 0.0) :`false` "/Game/Characters/Lena/Animations/GunIdle/FB_LenaGunIdle.FB_LenaGunIdle" :`true` "/Game/Characters/Lena/Animations/GunRunning/FB_LenaGunRunning.FB_LenaGunRunning" :!type "PaperFlipbook Object Reference") :`true` "/Game/Characters/Lena/Animations/GunFall/FB_LenaGunFall.FB_LenaGunFall"))
    (if (`self.DuckieDead`)
      (`SceneComponent.SetHiddenInGame` (`self.BP_Duckie`) true false))
    (else
      (`PaperFlipbookComponent.SetFlipbook` (`self.Sprite`) (select `bool` (`NavMovementComponent.IsFalling` (`self.CharacterMovement`)) :`false` (select `bool` (> (`KismetMathLibrary.VSize` (`MovementComponent.Velocity` (`self.CharacterMovement`))) 0.0) :`false` "/Game/Characters/Lena/Animations/Idle/FB_LenaIdleAnimation.FB_LenaIdleAnimation" :`true` "/Game/Characters/Lena/Animations/Running/FB_LenaRunningAnimation.FB_LenaRunningAnimation" :!type "PaperFlipbook Object Reference") :`true` "/Game/Characters/Lena/Animations/Falling/FB_LenaFall.FB_LenaFall"))
      (if (`self.DuckieDead`)
        (`SceneComponent.SetHiddenInGame` (`self.BP_Duckie`) true false)))))

(event `UpdateControlRotation`
  ;[1 1 1] animation controllers, rotation and contextual animations
  (`/Engine/EditorBlueprintResources/StandardMacros.IsValid` (`self.GetController`)
    (:`Is Valid`
      (`/Engine/EditorBlueprintResources/StandardMacros.CompareFloat` (`KismetMathLibrary.BreakVector3f` (`MovementComponent.Velocity` (`self.CharacterMovement`)))
        (:`>`
          (`Controller.SetControlRotation` (`self.GetController`) (`KismetMathLibrary.MakeRotator` 0.0)))
        (:`<`
          (`Controller.SetControlRotation` (`self.GetController`) (`KismetMathLibrary.MakeRotator` 0.0 0.0 180.0)))))))

(event `self.CapsuleComponent.OnComponentBeginOverlap`
  (params (OverlappedComponent :type "PrimitiveComponent Object Reference") (OtherActor :type "Actor Object Reference") (OtherComp :type "PrimitiveComponent Object Reference") (OtherBodyIndex :type Integer) (bFromSweep :type Boolean) (SweepResult :type "HitResult Structure (by ref)"))
  ;[1 1 1] GetKey For Level 1
  (if (== OtherActor "/Game/Actors/BP_Key.BP_Key")
    (set `self.HaveKey` true)))

(event `Key|E`
  (params (Key :type "Key Structure"))
  ;[1 1 1] Dialogue Mechanic - pls leave to ollie for now
  (:`Pressed`
    (for _array_element (`self.GetOverlappingActors` "/Game/Levels/Level_4/BP_Villager.BP_Villager_C")
      (if (`KismetSystemLibrary.DoesImplementInterface` _array_element "/Game/Levels/Level_4/BPI_VillagerDialogue.BPI_VillagerDialogue_C")
        (message `/Game/Levels/Level_4/BPI_VillagerDialogue.VillagerDialogue` _array_element)))))

(event `Key|E`
  (params (Key :type "Key Structure"))
  ;[1 1 1] Dialogue Mechanic - pls leave to ollie for now
  (:`Pressed`
    (for _array_element (`self.GetOverlappingActors` "/Game/Characters/Doux/Idle/BP_Doux.BP_Doux_C")
      (if (`KismetSystemLibrary.DoesImplementInterface` _array_element "/Game/Levels/Level_2/BPI_Doux.BPI_Doux_C")
        (set `self.TalkedToDOux` true)
        (message `/Game/Levels/Level_2/BPI_Doux.DouxDialogue` _array_element)))))

(fn `UserConstructionScript`)