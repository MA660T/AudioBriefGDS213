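; Checkpoint tracker actor that respawns the player at the active checkpoint, or at a PlayerStart when none is valid.
; Respawn triggers ResetPlayer, which briefly disables input, hides the player character and turns off its collision, then restores all three.
; Respawn's own matching delay runs in parallel before teleporting the pawn, so the move coincides with the character reappearing.
; ActiveCheckpoint is only read here, not assigned.
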(event `Respawn`
  (bind _returnvalue (`GameplayStatics.GetPlayerPawn` 0))
  (`self.Reset Player`)
  (`KismetSystemLibrary.Delay` 0.5)
  (`self.ActiveCheckpoint`
    (:`then`
      (`self.K2_SetActorLocation` _returnvalue (`self.K2_GetActorLocation` (`self.ActiveCheckpoint`)) false false))
    (:`else`
      (bind _returnvalue_2 (`GameplayStatics.GetActorOfClass` "/Script/Engine.PlayerStart"))
      (`self.K2_SetActorLocation` _returnvalue (`self.K2_GetActorLocation` _returnvalue_2) false false))))

(event `Reset Player`
  (bind _asbp_player_character (cast `/Game/Shared/Player/BP_PlayerCharacter` (`GameplayStatics.GetPlayerPawn` 0)))
  (`self.DisableInput` _asbp_player_character null)
  (`self.SetActorHiddenInGame` _asbp_player_character true)
  (`self.SetActorEnableCollision` _asbp_player_character false)
  (`KismetSystemLibrary.Delay` 0.5)
  (`self.SetActorHiddenInGame` _asbp_player_character false)
  (`self.EnableInput` _asbp_player_character null)
  (`self.SetActorEnableCollision` _asbp_player_character true))

(fn `UserConstructionScript`)