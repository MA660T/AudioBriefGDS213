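; Player character with single-axis movement along world X, wall sliding, wall jumping and a limited dash.
; While falling, a short forward trace each tick detects walls, turns the character to face them and interpolates its velocity to slide.
; Jump during a slide launches up and along fixed world -X.
; Dash launches along current X velocity up to twice, with the count resetting after a delay once grounded.
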(event `self.ReceiveTick`
  (params (DeltaSeconds :type "Float (single-precision)"))
  (bind _returnvalue (`self.K2_GetActorLocation`))
  (if (`NavMovementComponent.IsFalling` (`self.CharacterMovement`))
    (bind (_outhit _returnvalue_2) (`KismetSystemLibrary.LineTraceSingle` _returnvalue (+ _returnvalue (* (`self.GetActorForwardVector`) 70.0)) "TraceTypeQuery1"))
    (if _returnvalue_2
      (set `self.WallSlide` true)
      (bind (_returnvalue_roll _returnvalue_pitch _returnvalue_yaw) (`KismetMathLibrary.BreakRotator` (`KismetMathLibrary.Conv_VectorToRotator` (`.ImpactNormal` (`GameplayStatics.BreakHitResult` _outhit)))))
      (`self.K2_SetActorRotation` (`KismetMathLibrary.MakeRotator` 0.0 0.0 (+ _returnvalue_yaw 180.0)))
      (set `MovementComponent.Velocity` (`KismetMathLibrary.VInterpTo_Constant` (`self.GetVelocity`) (0.0 0.0 0.0) (`GameplayStatics.GetWorldDeltaSeconds`)) (`self.CharacterMovement`))
      (else
        (set `self.WallSlide` false :!label _label)))
    (else
      (goto _label))))

(event `InputAxis|Move Right`
  (params (AxisValue :type "Float (single-precision)"))
  (`self.AddMovementInput` (1.0 0.0 0.0) AxisValue)
  (`MovementComponent.SetPlaneConstraintFromVectors` (`self.CharacterMovement`) (0.0 0.0 0.0) (0.0 0.0 0.0)))

(event `InputAction|Jump`
  (params (Key :type "Key Structure"))
  (:`Pressed`
    (if (`self.WallSlide`)
      (`self.LaunchCharacter` (+ (* (`KismetMathLibrary.GetForwardVector` (struct)) -300.0) (0.0 0.0 800.0)))
      (else
        (`self.Jump`))))
  (:`Released`
    (`self.StopJumping`)))

(event `self.OnLanded`
  (params (Hit :type "HitResult Structure (by ref)"))
  (`KismetSystemLibrary.Delay` 0.01)
  (if (== (stale `InputAction|Dash` _result) 2) :!label _label_2
    (if (not (`NavMovementComponent.IsFalling` (`self.CharacterMovement`)))
      (`KismetSystemLibrary.Delay` 1.0)
      (set `self.DashCount` 0))))

(event `InputAction|Dash`
  (params (Key :type "Key Structure"))
  (bind _returnvalue_x (`KismetMathLibrary.BreakVector` (`self.GetVelocity`)))
  (:`Pressed`
    (if (!= (`self.DashCount`) 2)
      (`self.LaunchCharacter` (* (`KismetMathLibrary.MakeVector` _returnvalue_x) 2))
      (bind _result (`/Engine/EditorBlueprintResources/StandardMacros.IncrementInt` (`self.DashCount`))
        (:`  `
          (goto _label_2))))))

(fn `UserConstructionScript`)